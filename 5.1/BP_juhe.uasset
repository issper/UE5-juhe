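; Screen-space clustering (juhe) actor that declutters instances of JuheActor by hiding those that project close to one another.
; BeginPlay caches their actors and world locations and shows the mouse cursor; key 1, or Tick when TickDo is set, runs Juhe.
; Juhe repeatedly picks an unclustered actor as a visible representative, hiding others within JuheMinValue screen distance, until the processed count matches the list length.
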(event `self.ReceiveBeginPlay`
  (if (`KismetSystemLibrary.IsValidClass` (`self.juheActor`))
    (bind _outactors (`GameplayStatics.GetAllActorsOfClass` (`self.juheActor`)))
    (for _array_element _outactors
      (`KismetArrayLibrary.Array_Add` (`self.juheActorList`) (make `/Game/Struct_juhe` _array_element (`self.K2_GetActorLocation` _array_element))))
    (`KismetSystemLibrary.PrintString` (`KismetStringLibrary.Conv_IntToString` (`KismetArrayLibrary.Array_Length` _outactors)))
    (set `PlayerController.bShowMouseCursor` true (`GameplayStatics.GetPlayerController` 0))
    (else
      (set `PlayerController.bShowMouseCursor` true (`GameplayStatics.GetPlayerController` 0)))))

(event `Key|One`
  (params (Key :type "Key Structure"))
  (:`Pressed`
    (`self.juhe`)))

(event `self.ReceiveTick`
  (params (DeltaSeconds :type "Float (single-precision)"))
  (if (`self.tickDo`)
    (`self.juhe`)))

(fn `juhe`
  (locals (count :type Integer) (nowJuheActor :type "/Game/Struct_juhe Structure"))
  (bind (_nowjuheactor_actor _nowjuheactor_location _nowjuheactor_isjuhe _nowjuheactor_hasjuhe _nowjuheactor_scene) (break `/Game/Struct_juhe` (`local.nowJuheActor`)))
  (bind _juheactorlist (`self.juheActorList`))
  (bind (_nowjuheactor_actor_2 _nowjuheactor_location_2 _nowjuheactor_isjuhe_2) (break `/Game/Struct_juhe` (`local.nowJuheActor`)))
  (for (_ _array_index) _juheactorlist
    (setmembers `/Game/Struct_juhe` :`StructRef` (`|GetArrayItem` _juheactorlist _array_index) :`isJuhe` false :`hasJuhe` false))
  (for (_array_element _array_index_2) (`self.juheActorList`) :!label _label
    (if (or (`.isJuhe_5_16C8E620478B459E10F522A1B2E3AE4F` (break `/Game/Struct_juhe` _array_element)) (`.hasJuhe_7_17A8881844B57D8AECB195B01F118BCF` (break `/Game/Struct_juhe` _array_element)))
      _
      (elif _nowjuheactor_isjuhe_2
        (if (<= (`KismetMathLibrary.Distance2D` _nowjuheactor_scene (`PlayerController.ProjectWorldLocationToScreen` (`GameplayStatics.GetPlayerController` 0) (`.location_11_3DC1048541E31F9333D963A0B7D7724F` (break `/Game/Struct_juhe` _array_element)) true)) (`self.juheMinValue`))
          (setmembers `/Game/Struct_juhe` :`StructRef` (`|GetArrayItem` (`self.juheActorList`) _array_index_2) :`isJuhe` false :`hasJuhe` true)
          (`self.SetActorHiddenInGame` (break `/Game/Struct_juhe` _array_element) true)
          (set `local.count` (+ (`local.count`) 1) :!label _label_2))
        (else
          (set `local.nowJuheActor` (make `/Game/Struct_juhe` (break `/Game/Struct_juhe` _array_element) (0.0 0.0 0.0) true true (`PlayerController.ProjectWorldLocationToScreen` (`GameplayStatics.GetPlayerController` 0) (`.location_11_3DC1048541E31F9333D963A0B7D7724F` (break `/Game/Struct_juhe` _array_element)) true)))
          (setmembers `/Game/Struct_juhe` :`StructRef` (`|GetArrayItem` (`self.juheActorList`) _array_index_2) :`isJuhe` true :`hasJuhe` true)
          (`self.SetActorHiddenInGame` (break `/Game/Struct_juhe` _array_element) false)
          (goto _label_2)))))
  (set `local.nowJuheActor` (make `/Game/Struct_juhe` null))
  (if (not (== (`local.count`) (`KismetArrayLibrary.Array_Length` (`self.juheActorList`))))
    (goto _label)))

(fn `UserConstructionScript`)